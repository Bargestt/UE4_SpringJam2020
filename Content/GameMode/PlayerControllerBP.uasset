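; Player controller that handles keyboard shortcuts for the menu and a stats overlay.
; Escape casts the game mode to ForestGamemode and calls its ToggleMenu.
; F2 creates the Stats widget if it is not valid, then a FlipFlop alternates between adding it to the viewport and removing it.
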(event `Key|Escape`
  (params (Key :type "Key Structure"))
  (:`Pressed`
    (bind _asforest_gamemode (cast `/Game/GameMode/ForestGamemode` (`GameplayStatics.GetGameMode`)))
    (`/Game/GameMode/ForestGamemode.ToggleMenu` _asforest_gamemode)))

(event `Key|F2`
  (params (Key :type "Key Structure"))
  (bind _stats (`self.Stats`))
  (:`Pressed`
    (`self.Stats`
      (:`then`
        _)
      (:`else`
        (bind _returnvalue (`|CreateWidget` "/Game/GameMode/Stats.Stats_C"))
        (set `self.Stats` _returnvalue)))
    (`/Engine/EditorBlueprintResources/StandardMacros.FlipFlop`
      (:`A`
        (`UserWidget.AddToViewport` _stats 0))
      (:`B`
        (`Widget.RemoveFromParent` _stats)))))

(fn `UserConstructionScript`)